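; BP_BeamDoor is a holographic beam door that toggles between closed and open whenever one of its linked spatial buttons activates.
; On BeginPlay it binds to each button, creates a dynamic material and applies the optional start-open state.
; Two timelines animate fade and beam strength, with an FMOD sound on opening.
; The door opens by dropping its scene component far below after the fade, and closes by restoring it before reversing the fade.
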(event Custom|Pressed
  (bind _fadeemissive (Variables|Default|GetFadeEmissive))
  (bind _fadein (Variables|Default|GetFadeIn))
  (if (Variables|Default|GetIsA)
    (Variables|Default|SetIsA false)
    (Audio|Components|Audio|Play _fadein)
    (Audio|Components|Audio|Play _fadeemissive)
    (bind _returnvalue (Class|FMODBlueprintStatics|FindEventbyName "event:/SpatialPuzzles/A_Door_Hologram"))
    (Class|FMODBlueprintStatics|PlayEventatLocation _returnvalue (Math|Conversions|ToTransform(Vector) (Transformation|GetActorLocation)))
    (else
      (Transformation|SetWorldLocation (Variables|Default|GetScene) (Variables|Default|GetStartLoc) false)
      (Variables|Default|SetIsA true)
      (Utilities|String|Reverse _fadein)
      (Utilities|String|Reverse _fadeemissive))))

(event EventBeginPlay
  (Variables|Default|SetIsA true)
  (Variables|Default|SetStartLoc (Transformation|GetWorldLocation (Variables|Default|GetScene)))
  (for _array_element (Variables|Default|GetmButtonArray)
    (bind _asspatial_button_blueprint (Utilities|Casting|CastToSpatialButton_Blueprint _array_element))
    (EventDispatchers|BindEventtoSpatialButtonActivate _asspatial_button_blueprint (delegate Custom|Pressed))
    (bind _returnvalue (Rendering|Material|CreateDynamicMaterialInstance (Variables|Default|GetRight) 0 0 :!class /Script/Engine.PrimitiveComponent))
    (Variables|Default|SetRightMat _returnvalue)
    (if (Variables|Default|GetmStartOpen)
      (Transformation|SetRelativeLocation (Variables|Default|GetScene) "0, 0,-3000.000000" false)
      (Utilities|String|Reverse (Variables|Default|GetFadeIn))
      (Utilities|String|Reverse (Variables|Default|GetFadeEmissive))
      (Variables|Default|SetIsA false))))

(fn ConstructionScript)