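; Clickable 3D rune button for the main menu that plays, opens options, or quits the game, depending on its Play, Options and Exit flags.
; A dynamic material instance toggles a highlight on cursor hover unless InMenu is set.
; Play opens the menu game mode's default level and Options adds a widget, each triggering a UI sound event.
; Opening Options also sets InMenu on every rune, suppressing further hover changes.
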(event EventActorBeginCursorOver
  (if (not (Variables|Default|GetInMenu))
    (Rendering|Material|SetScalarParameterValue (Variables|Default|GetMat_Inst) "HighlightOn" 1.0 :!class /Script/Engine.MaterialInstanceDynamic)))

(event EventActorEndCursorOver
  (if (not (Variables|Default|GetInMenu))
    (Rendering|Material|SetScalarParameterValue (Variables|Default|GetMat_Inst) "HighlightOn" 0.0 :!class /Script/Engine.MaterialInstanceDynamic)))

(event EventActorOnClicked
  (if (Variables|Default|GetPlay)
    (bind _asmenu_mode_blueprint (Utilities|Casting|CastToMenuMode_blueprint (Game|GetGameMode)))
    (Game|OpenLevel(byName) 0 (Variables|/Script/Above.MenuMode|GetDefaultLevel _asmenu_mode_blueprint))
    (bind _returnvalue (Class|FMODBlueprintStatics|FindEventbyName "event:/UI/UI_Play"))
    (Class|FMODBlueprintStatics|PlayEvent2D _returnvalue)
    (elif (Variables|Default|GetOptions)
      (bind _returnvalue_2 (UserInterface|CreateWidget "/Game/Blueprints/Menus/Option.Option_C"))
      (UserInterface|Viewport|AddtoViewport _returnvalue_2 0)
      (bind _returnvalue_3 (Class|FMODBlueprintStatics|FindEventbyName "event:/UI/UI_Button"))
      (Class|FMODBlueprintStatics|PlayEvent2D _returnvalue_3)
      (bind _outactors (Actor|GetAllActorsOfClass 0 "Menu_Rune_C"))
      (for _array_element _outactors
        (bind _asmenu_rune (Utilities|Casting|CastToMenu_Rune _array_element))
        (Variables|Menu_Rune_C|SetInMenu _asmenu_rune true)
        (Rendering|Material|SetScalarParameterValue (Variables|Default|GetMat_Inst) "HighlightOn" 0.0 :!class /Script/Engine.MaterialInstanceDynamic))
      (elif (Variables|Default|GetExit)
        (Game|QuitGame 0 0 "Quit")))))

(event EventBeginPlay
  (bind _returnvalue (Rendering|Material|CreateDynamicMaterialInstance (Variables|Debug|GetStaticMeshComponent) 0 0 :!class /Script/Engine.PrimitiveComponent))
  (bind _output_get (Variables|Default|SetMat_Inst _returnvalue))
  (Rendering|Material|SetScalarParameterValue _output_get "HighlightSize" 3.0 :!class /Script/Engine.MaterialInstanceDynamic)
  (Rendering|Material|SetScalarParameterValue _output_get "Contrast" 0.3 :!class /Script/Engine.MaterialInstanceDynamic))

(fn ConstructionScript)