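; End-of-level trigger that starts the game mode's end sequence from an interaction button and drives a color effect.
; Pressing the child Trigger calls AboveGameMode's EndTrigger, brightens the beam and light, and enables the ColorTint post-process it registered at BeginPlay.
; A later overlap destroys the old battery and creates a dynamic instance of the first blendable.
; Tick then lerps its ColorStr and the color grading intensity toward full, debug-printing each frame.
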(event Custom|Pressed
  (bind _pointlight (Variables|Default|GetPointLight))
  ;[1 1 1] Activation Button
  (bind _asabove_game_mode (Utilities|Casting|CastToAboveGameMode (Variables|/Script/Engine.GameState|GetAuthorityGameMode (Game|GetGameState))))
  (Class|AboveGameMode|EndTrigger _asabove_game_mode (Game|GetPlayerCharacter 0) (Variables|Default|GetOldBattery) (Variables|Default|GetBox))
  (Variables|Default|SetPresed true)
  ;[1 1 1] Make the beam light brighter
  (Variables|/Script/Engine.PostProcessComponent|SetbEnabled (Variables|Default|GetColorTint) true)
  (bind _returnvalue (Rendering|Material|CreateDynamicMaterialInstance (Variables|Default|GetBeam) 0 "/Game/Materials/Beam_Mater.Beam_Mater" :!class /Script/Engine.PrimitiveComponent))
  (Rendering|Material|SetScalarParameterValue _returnvalue "BeamStrength" 1e+02 :!class /Script/Engine.MaterialInstanceDynamic)
  (Variables|/Script/Engine.PostProcessComponent|SetBlendWeight (Variables|Default|GetColorTint) 1.0)
  (Rendering|Components|Light|SetIntensity _pointlight (+ (Variables|/Script/Engine.LightComponentBase|GetIntensity _pointlight) 2e+04)))

(event EventTick
  (params (DeltaSeconds :type Float%20%28single-precision%29))
  (bind _colortint (Variables|Default|GetColorTint))
  (bind _helper (Variables|Default|GetHelper))
  (bind _settings (Variables|/Script/Engine.PostProcessComponent|GetSettings _colortint))
  (bind (_boverride_filmwhitepoint _boverride_filmsaturation _boverride_filmchannelmixerred _boverride_filmchannelmixergreen _boverride_filmchannelmixerblue _boverride_filmcontrast _boverride_filmdynamicrange _boverride_filmhealamount _boverride_filmtoeamount _boverride_filmshadowtint _boverride_filmshadowtintblend _boverride_filmshadowtintamount _boverride_scenecolortint _boverride_scenefringeintensity _boverride_scenefringesaturation _boverride_ambientcubemaptint _boverride_ambientcubemapintensity _boverride_bloomintensity _boverride_bloomthreshold _boverride_bloom1tint _boverride_bloom1size _boverride_bloom2size _boverride_bloom2tint _boverride_bloom3tint _boverride_bloom3size _boverride_bloom4tint _boverride_bloom4size _boverride_bloom5tint _boverride_bloom5size _boverride_bloomdirtmaskintensity _boverride_bloomdirtmasktint _boverride_bloomdirtmask _boverride_autoexposurelowpercent _boverride_autoexposurehighpercent _boverride_autoexposureminbrightness _boverride_autoexposuremaxbrightness _boverride_autoexposurespeedup _boverride_autoexposurespeeddown _boverride_autoexposurebias _boverride_histogramlogmin _boverride_histogramlogmax _boverride_lensflareintensity _boverride_lensflaretint _boverride_lensflaretints _boverride_lensflarebokehsize _boverride_lensflarebokehshape _boverride_lensflarethreshold _boverride_vignetteintensity _boverride_vignettecolor _boverride_grainintensity _boverride_grainjitter _boverride_ambientocclusionintensity _boverride_ambientocclusionstaticfraction _boverride_ambientocclusionradius _boverride_ambientocclusionfadedistance _boverride_ambientocclusionfaderadius _boverride_ambientocclusiondistance _boverride_ambientocclusionradiusinws _boverride_ambientocclusionpower _boverride_ambientocclusionbias _boverride_ambientocclusionquality _boverride_ambientocclusionmipblend _boverride_ambientocclusionmipscale _boverride_ambientocclusionmipthreshold _boverride_lpvintensity _boverride_lpvwarpintensity _boverride_lpvsize _boverride_lpvsecondaryocclusionintensity _boverride_lpvsecondarybounceintensity _boverride_lpvgeometryvolumebias _boverride_lpvvplinjectionbias _boverride_lpvemissiveinjectionintensity _boverride_lpvtransmissionintensity _boverride_indirectlightingcolor _boverride_indirectlightingintensity _boverride_colorgradingintensity _boverride_colorgradinglut _boverride_depthoffieldfocaldistance _boverride_depthoffieldfocalregion _boverride_depthoffieldneartransitionregion _boverride_depthoffieldfartransitionregion _boverride_depthoffieldscale _boverride_depthoffieldmaxbokehsize _boverride_depthoffieldnearblursize _boverride_depthoffieldfarblursize _boverride_depthoffieldmethod _boverride_depthoffieldbokehshape _boverride_depthoffieldocclusion _boverride_depthoffieldcolorthreshold _boverride_depthoffieldsizethreshold _boverride_depthoffieldskyfocusdistance _boverride_motionbluramount _boverride_motionblurmax _boverride_motionblurperobjectsize _boverride_screenpercentage _boverride_antialiasingmethod _boverride_screenspacereflectionintensity _boverride_screenspacereflectionquality _boverride_screenspacereflectionmaxroughness _boverride_screenspacereflectionroughnessscale _filmwhitepoint _filmshadowtint _filmshadowtintblend _filmshadowtintamount _filmsaturation _filmchannelmixerred _filmchannelmixergreen _filmchannelmixerblue _filmcontrast _filmtoeamount _filmhealamount _filmdynamicrange _scenecolortint _scenefringeintensity _scenefringesaturation _bloomintensity _bloomthreshold _bloom1size _bloom2size _bloom3size _bloom4size _bloom5size _bloom1tint _bloom2tint _bloom3tint _bloom4tint _bloom5tint _bloomdirtmaskintensity _bloomdirtmasktint _bloomdirtmask _lpvintensity _lpvwarpintensity _lpvvplinjectionbias _lpvsize _lpvsecondaryocclusionintensity _lpvsecondarybounceintensity _lpvgeometryvolumebias _lpvemissiveinjectionintensity _lpvtransmissionintensity _ambientcubemaptint _ambientcubemapintensity _ambientcubemap _autoexposurelowpercent _autoexposurehighpercent _autoexposureminbrightness _autoexposuremaxbrightness _autoexposurespeedup _autoexposurespeeddown _autoexposurebias _histogramlogmin _histogramlogmax _lensflareintensity _lensflaretint _lensflarebokehsize _lensflarethreshold _lensflarebokehshape _lensflaretints _vignetteintensity _vignettecolor _grainjitter _grainintensity _ambientocclusionintensity _ambientocclusionstaticfraction _ambientocclusionradius _ambientocclusionradiusinws _ambientocclusionfadedistance _ambientocclusionfaderadius _ambientocclusiondistance _ambientocclusionpower _ambientocclusionbias _ambientocclusionquality _ambientocclusionmipblend _ambientocclusionmipscale _ambientocclusionmipthreshold _indirectlightingcolor _indirectlightingintensity _colorgradingintensity _colorgradinglut _depthoffieldmethod _depthoffieldfocaldistance _depthoffieldfocalregion _depthoffieldneartransitionregion _depthoffieldfartransitionregion _depthoffieldscale _depthoffieldmaxbokehsize _depthoffieldnearblursize _depthoffieldfarblursize _depthoffieldbokehshape _depthoffieldocclusion _depthoffieldcolorthreshold _depthoffieldsizethreshold _depthoffieldskyfocusdistance _motionbluramount _motionblurmax _motionblurperobjectsize _screenpercentage _antialiasingmethod _screenspacereflectionintensity _screenspacereflectionquality _screenspacereflectionmaxroughness _blendables) (Utilities|Struct|BreakPostProcessSettings _settings))
  (if (Variables|Default|GetNewBattery)
    (bind _output_get (Variables|Default|SetmCurrentExpose (Math|Float|Lerp (Variables|Default|GetmCurrentExpose) 1.0 0.2)))
    (Rendering|Material|SetScalarParameterValue _helper "ColorStr" _output_get :!class /Script/Engine.MaterialInstanceDynamic)
    (bind _returnvalue (Rendering|Material|GetScalarParameterValue _helper "ColorStr" :!class /Script/Engine.MaterialInstanceDynamic))
    (Development|PrintString (Utilities|String|ToString(Float) _returnvalue))
    (Utilities|Struct|SetmembersinPostProcessSettings _settings _boverride_filmwhitepoint _boverride_filmsaturation _boverride_filmchannelmixerred _boverride_filmchannelmixergreen _boverride_filmchannelmixerblue _boverride_filmcontrast _boverride_filmdynamicrange _boverride_filmhealamount _boverride_filmtoeamount _boverride_filmshadowtint _boverride_filmshadowtintblend _boverride_filmshadowtintamount _boverride_scenecolortint _boverride_scenefringeintensity _boverride_scenefringesaturation _boverride_ambientcubemaptint _boverride_ambientcubemapintensity _boverride_bloomintensity _boverride_bloomthreshold _boverride_bloom1tint _boverride_bloom1size _boverride_bloom2size _boverride_bloom2tint _boverride_bloom3tint _boverride_bloom3size _boverride_bloom4tint _boverride_bloom4size _boverride_bloom5tint _boverride_bloom5size _boverride_bloomdirtmaskintensity _boverride_bloomdirtmasktint _boverride_bloomdirtmask _boverride_autoexposurelowpercent _boverride_autoexposurehighpercent _boverride_autoexposureminbrightness _boverride_autoexposuremaxbrightness _boverride_autoexposurespeedup _boverride_autoexposurespeeddown _boverride_autoexposurebias _boverride_histogramlogmin _boverride_histogramlogmax _boverride_lensflareintensity _boverride_lensflaretint _boverride_lensflaretints _boverride_lensflarebokehsize _boverride_lensflarebokehshape _boverride_lensflarethreshold _boverride_vignetteintensity _boverride_vignettecolor _boverride_grainintensity _boverride_grainjitter _boverride_ambientocclusionintensity _boverride_ambientocclusionstaticfraction _boverride_ambientocclusionradius _boverride_ambientocclusionfadedistance _boverride_ambientocclusionfaderadius _boverride_ambientocclusiondistance _boverride_ambientocclusionradiusinws _boverride_ambientocclusionpower _boverride_ambientocclusionbias _boverride_ambientocclusionquality _boverride_ambientocclusionmipblend _boverride_ambientocclusionmipscale _boverride_ambientocclusionmipthreshold _boverride_lpvintensity _boverride_lpvwarpintensity _boverride_lpvsize _boverride_lpvsecondaryocclusionintensity _boverride_lpvsecondarybounceintensity _boverride_lpvgeometryvolumebias _boverride_lpvvplinjectionbias _boverride_lpvemissiveinjectionintensity _boverride_lpvtransmissionintensity _boverride_indirectlightingcolor _boverride_indirectlightingintensity _boverride_colorgradingintensity _boverride_colorgradinglut _boverride_depthoffieldfocaldistance _boverride_depthoffieldfocalregion _boverride_depthoffieldneartransitionregion _boverride_depthoffieldfartransitionregion _boverride_depthoffieldscale _boverride_depthoffieldmaxbokehsize _boverride_depthoffieldnearblursize _boverride_depthoffieldfarblursize _boverride_depthoffieldmethod _boverride_depthoffieldbokehshape _boverride_depthoffieldocclusion _boverride_depthoffieldcolorthreshold _boverride_depthoffieldsizethreshold _boverride_depthoffieldskyfocusdistance _boverride_motionbluramount _boverride_motionblurmax _boverride_motionblurperobjectsize _boverride_screenpercentage _boverride_antialiasingmethod _boverride_screenspacereflectionintensity _boverride_screenspacereflectionquality _boverride_screenspacereflectionmaxroughness _boverride_screenspacereflectionroughnessscale _filmwhitepoint _filmshadowtint _filmshadowtintblend _filmshadowtintamount _filmsaturation _filmchannelmixerred _filmchannelmixergreen _filmchannelmixerblue _filmcontrast _filmtoeamount _filmhealamount _filmdynamicrange _scenecolortint _scenefringeintensity _scenefringesaturation _bloomintensity _bloomthreshold _bloom1size _bloom2size _bloom3size _bloom4size _bloom5size _bloom1tint _bloom2tint _bloom3tint _bloom4tint _bloom5tint _bloomdirtmaskintensity _bloomdirtmasktint _bloomdirtmask _lpvintensity _lpvwarpintensity _lpvvplinjectionbias _lpvsize _lpvsecondaryocclusionintensity _lpvsecondarybounceintensity _lpvgeometryvolumebias _lpvemissiveinjectionintensity _lpvtransmissionintensity _ambientcubemaptint _ambientcubemapintensity _ambientcubemap _autoexposurelowpercent _autoexposurehighpercent _autoexposureminbrightness _autoexposuremaxbrightness _autoexposurespeedup _autoexposurespeeddown 0.0 _histogramlogmin _histogramlogmax _lensflareintensity _lensflaretint _lensflarebokehsize _lensflarethreshold _lensflarebokehshape _vignetteintensity _vignettecolor _grainjitter _grainintensity _ambientocclusionintensity _ambientocclusionstaticfraction _ambientocclusionradius _ambientocclusionradiusinws _ambientocclusionfadedistance _ambientocclusionfaderadius _ambientocclusiondistance _ambientocclusionpower _ambientocclusionbias _ambientocclusionquality _ambientocclusionmipblend _ambientocclusionmipscale _ambientocclusionmipthreshold _indirectlightingcolor _indirectlightingintensity (Variables|Default|GetmCurrentExpose) _colorgradinglut _depthoffieldmethod _depthoffieldfocaldistance _depthoffieldfocalregion _depthoffieldneartransitionregion _depthoffieldfartransitionregion _depthoffieldscale _depthoffieldmaxbokehsize _depthoffieldnearblursize _depthoffieldfarblursize _depthoffieldbokehshape _depthoffieldocclusion _depthoffieldcolorthreshold _depthoffieldsizethreshold _depthoffieldskyfocusdistance _motionbluramount _motionblurmax _motionblurperobjectsize _screenpercentage _antialiasingmethod _screenspacereflectionintensity _screenspacereflectionquality _screenspacereflectionmaxroughness _blendables)))

(event EventBeginPlay
  ;[1 1 1] Activation Button
  (Variables|/Script/Engine.PostProcessComponent|SetbEnabled (Variables|Default|GetColorTint) false)
  (bind _asinteraction_trigger_blueprint (Utilities|Casting|CastToInteraction_Trigger_Blueprint (Variables|/Script/Engine.ChildActorComponent|GetChildActor (Variables|Default|GetTrigger))))
  (EventDispatchers|BindEventtoInteractionDispatcher _asinteraction_trigger_blueprint (delegate Custom|Pressed))
  (bind _asabove_game_mode (Utilities|Casting|CastToAboveGameMode (Variables|/Script/Engine.GameState|GetAuthorityGameMode (Game|GetGameState))))
  (Variables|/Script/Above.AboveGameMode|SetmPostProcess _asabove_game_mode (Variables|Default|GetColorTint)))

(event EventActorBeginOverlap
  (params (OtherActor :type Actor%20Object%20Reference))
  ;[1 1 1] Stand on End box
  (if (Variables|Default|GetPresed)
    (Components|DestroyComponent (Variables|Default|GetOldBattery))
    (Variables|Default|SetNewBattery true)
    (Variables|/Script/Engine.PostProcessComponent|SetbEnabled (Variables|Default|GetColorTint) true)
    (bind _asmaterial_instance (Utilities|Casting|CastToMaterialInstance (Utilities|Array|Get(acopy) (.Blendables (Utilities|Struct|BreakPostProcessSettings (Variables|/Script/Engine.PostProcessComponent|GetSettings (Variables|Default|GetColorTint)))))))
    (bind _returnvalue (Rendering|Material|CreateDynamicMaterialInstance _asmaterial_instance :!class /Script/Engine.KismetMaterialLibrary))
    (Variables|Default|SetHelper _returnvalue)))

(fn ConstructionScript)