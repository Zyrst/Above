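; Cloud actor with outer, middle and inner layer components, apparently meant to rotate the inner layer.
; The construction script assigns the three components to OuterClouds, MiddleClouds and InnerClouds variables.
; A disconnected chain would add to the inner layer's pitch by scaled delta time, but it never runs.
; BeginPlay, Tick and the RotateInner event are empty, so the event graph does nothing at runtime.
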(event Custom|Rotate%20Inner)

(event EventBeginPlay)

(event EventActorBeginOverlap
  (params (OtherActor :type Actor%20Object%20Reference)))

(event EventTick
  (params (DeltaSeconds :type Float%20%28single-precision%29)))

(fn ConstructionScript
  (Variables|Default|SetOuterClouds (Variables|Default|GetOuter))
  (Variables|Default|SetMiddleClouds (Variables|Default|GetMiddle))
  (Variables|Default|SetInnerClouds (Variables|Default|GetInner)))