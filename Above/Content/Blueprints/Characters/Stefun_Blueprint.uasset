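; Character Blueprint for Stefun that drives its FMOD audio: ambience/music and movement sound.
; BeginPlay starts the 2D AMBMUS event, and SoundEventParameterChange writes a named parameter to that instance.
; Move events start the Movement event at the actor's current location, feed it a Speed parameter from GetMoveSpeed, and stop it.
; The movement instance is placed at its start location rather than attached to the actor.
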(event EventSoundEventEndMove
  ;[1 1 1] Audio events
  (Class|FMODBlueprintStatics|EventInstanceStop (stale EventSoundEventBeginMove _returnvalue_2)))

(event EventSoundEventMove
  ;[1 1 1] Audio events
  (bind _returnvalue (Class|Stefun|GetMoveSpeed))
  (Class|FMODBlueprintStatics|EventInstanceSetParameter (stale EventSoundEventBeginMove _returnvalue_2) "Speed" _returnvalue))

(event EventSoundEventParameterChange
  ;[1 1 1] Audio events
  (Class|FMODBlueprintStatics|EventInstanceSetParameter (stale EventBeginPlay _returnvalue_2) (Variables|Default|GetmParameterChangeName) (Variables|Default|GetmParameterChangeValue)))

(event EventBeginPlay
  ;[1 1 1] Audio events
  (bind _returnvalue (Class|FMODBlueprintStatics|FindEventbyName "event:/AMBMUS"))
  (bind _returnvalue_2 (Class|FMODBlueprintStatics|PlayEvent2D _returnvalue)))

(event EventSoundEventBeginMove
  ;[1 1 1] Audio events
  (bind _returnvalue (Class|FMODBlueprintStatics|FindEventbyName "event:/Movement"))
  (bind _returnvalue_2 (Class|FMODBlueprintStatics|PlayEventatLocation _returnvalue (Math|Conversions|ToTransform(Vector) (Transformation|GetActorLocation)))))

(fn ConstructionScript)