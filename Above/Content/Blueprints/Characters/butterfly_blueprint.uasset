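; Butterfly actor whose construction script randomizes its look.
; It adds one of two skeletal mesh components at random, each at the actor's origin with a random rotation without roll.
; A random animation rate scale is applied only to the first component variant.
; A random pick then sets the default, blue or pink butterfly material on both component references, though only one is created per run.
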(fn ConstructionScript
  (bind _returnvalue (Math|Random|RandomRotator false))
  (bind _returnvalue_2 (Math|Transform|MakeTransform "0, 0, 0" _returnvalue))
  (if (Math|Random|RandomBool)
    (bind _returnvalue_3 (AddComponent|AddSkeletalMeshComponent false _returnvalue_2))
    (else
      (bind _returnvalue_4 (AddComponent|AddSkeletalMeshComponent false _returnvalue_2))))
  (Variables|/Script/Engine.SkeletalMeshComponent|SetGlobalAnimRateScale _returnvalue_3 (Math|Random|RandomFloatinRange 0.5 1.5))
  (switch int (Math|Random|RandomInteger 3)
    (:Default
      (Rendering|Material|SetMaterial _returnvalue_4 0 "/Game/Models_and_textures/Creatures/Butterflies/Enviroment/Textures/Texture_Butterfly_Mat.Texture_Butterfly_Mat" :!label _label))
    (:0
      (Rendering|Material|SetMaterial _returnvalue_3 0 "/Game/Models_and_textures/Creatures/Butterflies/Enviroment/Textures/texture_butterfly_blue_Mat.texture_butterfly_blue_Mat"))
    (:1
      (Rendering|Material|SetMaterial _returnvalue_4 0 "/Game/Models_and_textures/Creatures/Butterflies/Enviroment/Textures/texture_butterfly_pink_Mat.texture_butterfly_pink_Mat"))
    (:2
      (goto _label))))