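; Interactable trigger that activates directly on interaction, or on completion of a linked color puzzle.
; BeginPlay binds to the child interaction trigger and puzzle dispatchers, then assigns the highlight material and puzzle reference, both skipped without a color puzzle.
; Interact always fires its dispatcher but calls Activate only when no puzzle reference is valid.
; The construction script creates a dynamic material instance on the model.
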(event Custom|Interact
  (if (Utilities|IsValid (Variables|Default|GetpuzzleReference))
    _
    (else
      (Class|KanelbulleTrigger|Activate)))
  (Default|CallInteractDispatcher))

(event Custom|ColorPuzzle
  (Class|KanelbulleTrigger|Activate))

(event EventBeginPlay
  (bind _asinteraction_trigger_blueprint (Utilities|Casting|CastToInteraction_Trigger_Blueprint (Variables|/Script/Engine.ChildActorComponent|GetChildActor (Variables|Default|GetInteraction_Trigger_Blueprint))))
  (EventDispatchers|BindEventtoInteractionDispatcher _asinteraction_trigger_blueprint (delegate Custom|Interact))
  (bind _ascolor_puzzle_blueprint (Utilities|Casting|CastToColor_Puzzle_Blueprint (Variables|Default|GetmColorPuzzleReference)))
  (EventDispatchers|BindEventtoPuzzleDoneDispatcher _ascolor_puzzle_blueprint (delegate Custom|ColorPuzzle))
  (CallFunction|AssignHighlightMaterial (Variables|Default|GetModel_mekaniksak) _asinteraction_trigger_blueprint)
  (Variables|Default|SetpuzzleReference (Variables|Default|GetmColorPuzzleReference)))

(event EventActorBeginOverlap
  (params (OtherActor :type Actor%20Object%20Reference)))

(event EventTick
  (params (DeltaSeconds :type Float%20%28single-precision%29)))

(fn ConstructionScript
  (bind _returnvalue (Rendering|Material|CreateDynamicMaterialInstance (Variables|Default|GetModel_mekaniksak) 0 0 :!class /Script/Engine.PrimitiveComponent))
  (Variables|Default|SetmMaterial _returnvalue))