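; Trigger volume that changes a named sound parameter when a Stefun_Blueprint actor enters or leaves it.
; BeginPlay binds overlap events on the box, sphere or capsule collider chosen by MColliderType.
; Overlaps feed ParameterChangeEnter and ParameterChangeExit, which cast the actor and call its ChangeParameter with separate enter and exit name/value pairs.
; The sphere's end-overlap binding is unconnected, so sphere triggers only apply the enter change.
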(event Custom|OverlapEndBox
  (params (OtherActor :type Actor%20Object%20Reference) (OtherComp :type Primitive%20Component%20Object%20Reference) (OtherBodyIndex :type Integer))
  (CallFunction|ParameterChangeExit OtherActor))

(event Custom|OverlapEndCapsule
  (params (OtherActor :type Actor%20Object%20Reference) (OtherComp :type Primitive%20Component%20Object%20Reference) (OtherBodyIndex :type Integer))
  (CallFunction|ParameterChangeExit OtherActor))

(event Custom|OverlapSpehere
  (params (OtherActor :type Actor%20Object%20Reference) (OtherComp :type Primitive%20Component%20Object%20Reference) (OtherBodyIndex :type Integer) (bFromSweep :type Boolean) (SweepResult :type Hit%20Result%20Structure%20%28by%20ref%29))
  (CallFunction|ParameterChangeEnter OtherActor))

(event Custom|OverlapCapsule
  (params (OtherActor :type Actor%20Object%20Reference) (OtherComp :type Primitive%20Component%20Object%20Reference) (OtherBodyIndex :type Integer) (bFromSweep :type Boolean) (SweepResult :type Hit%20Result%20Structure%20%28by%20ref%29))
  (CallFunction|ParameterChangeEnter OtherActor))

(event Custom|OverlapBox
  (params (OtherActor :type Actor%20Object%20Reference) (OtherComp :type Primitive%20Component%20Object%20Reference) (OtherBodyIndex :type Integer) (bFromSweep :type Boolean) (SweepResult :type Hit%20Result%20Structure%20%28by%20ref%29))
  (CallFunction|ParameterChangeEnter OtherActor))

(event Custom|OverlapEndSphere
  (params (OtherActor :type Actor%20Object%20Reference) (OtherComp :type Primitive%20Component%20Object%20Reference) (OtherBodyIndex :type Integer))
  (CallFunction|ParameterChangeExit OtherActor))

(event EventBeginPlay
  (bind _boxcollider (Variables|Default|GetBoxCollider))
  (bind _capsulecollider (Variables|Default|GetCapsuleCollider))
  (switch Utilities|FlowControl|Switch|SwitchonColliderType (Variables|Default|GetmColliderType)
    (:Box
      (Collision|BindEventtoOnComponentBeginOverlap _boxcollider (delegate Custom|OverlapSpehere))
      (Collision|AssignOnComponentEndOverlap _boxcollider (delegate Custom|OverlapEndBox)))
    (:Spehere
      (Collision|BindEventtoOnComponentBeginOverlap (Variables|Default|GetSphereCollider) (delegate Custom|OverlapBox)))
    (:Capsule
      (Collision|BindEventtoOnComponentBeginOverlap _capsulecollider (delegate Custom|OverlapCapsule))
      (Collision|AssignOnComponentEndOverlap _capsulecollider (delegate Custom|OverlapEndCapsule)))))

(event EventTick
  (params (DeltaSeconds :type Float%20%28single-precision%29)))

(fn ConstructionScript)

(fn ParameterChangeExit
  (params (Actor :type Object%20Object%20Reference))
  (bind _asstefun_blueprint (Utilities|Casting|CastToStefun_Blueprint Actor))
  (Class|Stefun|ChangeParameter _asstefun_blueprint (Variables|Default|GetmExitParameterName) (Variables|Default|GetmExitParameterValue))
  (return))

(fn ParameterChangeEnter
  (params (Actor :type Object%20Object%20Reference))
  (bind _asstefun_blueprint (Utilities|Casting|CastToStefun_Blueprint Actor))
  (Class|Stefun|ChangeParameter _asstefun_blueprint (Variables|Default|GetmEnterParameterName) (Variables|Default|GetmEnterParameterValue))
  (return))