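; Sound trigger Blueprint that changes music parameters on the Stefun_Blueprint actor.
; OnOverlapBeginEvent acts only with EndTrigger set: a zero enter value plays last-room music, any other changes that music's parameter.
; Box, sphere and capsule overlap handlers forward configured enter and exit name/value pairs to ChangeParameter.
; The collider-type switch that binds those handlers is unconnected, so this graph never binds them.
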(event Custom|OverlapEndBox
  (params (OtherActor :type Actor%20Object%20Reference) (OtherComp :type Primitive%20Component%20Object%20Reference) (OtherBodyIndex :type Integer))
  (CallFunction|ParameterChangeExit OtherActor))

(event Custom|OverlapEndCapsule
  (params (OtherActor :type Actor%20Object%20Reference) (OtherComp :type Primitive%20Component%20Object%20Reference) (OtherBodyIndex :type Integer))
  (CallFunction|ParameterChangeExit OtherActor))

(event Custom|OverlapSpehere
  (params (OtherActor :type Actor%20Object%20Reference) (OtherComp :type Primitive%20Component%20Object%20Reference) (OtherBodyIndex :type Integer) (bFromSweep :type Boolean) (SweepResult :type Hit%20Result%20Structure%20%28by%20ref%29))
  (CallFunction|ParameterChangeEnter OtherActor))

(event Custom|OverlapCapsule
  (params (OtherActor :type Actor%20Object%20Reference) (OtherComp :type Primitive%20Component%20Object%20Reference) (OtherBodyIndex :type Integer) (bFromSweep :type Boolean) (SweepResult :type Hit%20Result%20Structure%20%28by%20ref%29))
  (CallFunction|ParameterChangeEnter OtherActor))

(event Custom|OverlapBox
  (params (OtherActor :type Actor%20Object%20Reference) (OtherComp :type Primitive%20Component%20Object%20Reference) (OtherBodyIndex :type Integer) (bFromSweep :type Boolean) (SweepResult :type Hit%20Result%20Structure%20%28by%20ref%29))
  (CallFunction|ParameterChangeEnter OtherActor))

(event Custom|OverlapEndSphere
  (params (OtherActor :type Actor%20Object%20Reference) (OtherComp :type Primitive%20Component%20Object%20Reference) (OtherBodyIndex :type Integer))
  (CallFunction|ParameterChangeExit OtherActor))

(event EventBeginPlay)

(event EventTick
  (params (DeltaSeconds :type Float%20%28single-precision%29)))

(event EventOnOverlapBeginEvent
  (params (stefun :type Stefun%20Object%20Reference))
  (if (Variables|Default|GetEndTrigger)
    (bind _asstefun_blueprint (Utilities|Casting|CastToStefun_Blueprint stefun))
    (if (== (Variables|Default|GetmEnterParameterValue) 0.0)
      (Default|PlayLastRoomMusic _asstefun_blueprint)
      (else
        (Default|LastRoomMusicParameterChange _asstefun_blueprint (Variables|Default|GetmEnterParameterValue))))))

(fn ConstructionScript)

(fn ParameterChangeExit
  (params (Actor :type Object%20Object%20Reference))
  (bind _asstefun_blueprint (Utilities|Casting|CastToStefun_Blueprint Actor))
  (Class|Stefun|ChangeParameter _asstefun_blueprint (Variables|Default|GetmExitParameterName) (Variables|Default|GetmExitParameterValue))
  (return))

(fn ParameterChangeEnter
  (params (Actor :type Object%20Object%20Reference))
  (bind _asstefun_blueprint (Utilities|Casting|CastToStefun_Blueprint Actor))
  (Class|Stefun|ChangeParameter _asstefun_blueprint (Variables|Default|GetmEnterParameterName) (Variables|Default|GetmEnterParameterValue))
  (return))